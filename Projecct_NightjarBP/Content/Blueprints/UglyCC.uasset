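; UglyCC is the player character, a brawler that fights BP_CanardRaciste enemies and tracks its kills and life.
; Melee plays a punch montage, then a delayed forward sphere trace calls GetHit on the enemy it finds.
; Grab and throw inputs share one montage-only branch picked by IsGrabbingEnemy, with flags blocking replays.
; At zero life, it shows the end-game widget and mouse cursor and calls GameOver on every enemy.
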(event Custom|Kill
  (Variables|Default|SetKiilCount (+ (Variables|Default|GetKiilCount) 1)))

(event Custom|Get%20HIt
  (bind _returnvalue (Game|GetPlayerController 0))
  (Variables|Default|SetLife (- (Variables|Default|GetLife) 1))
  (if (== (Variables|Default|GetLife) 0)
    (bind _returnvalue_2 (UserInterface|CreateWidget "/Game/UI/WBP_EndGame.WBP_EndGame_C" _returnvalue))
    (UserInterface|Viewport|AddtoViewport _returnvalue_2 0)
    (Variables|/Script/Engine.PlayerController|SetbShowMouseCursor _returnvalue true)
    (bind _outactors (Actor|GetAllActorsOfClass "/Game/AI/BP_CanardRaciste.BP_CanardRaciste_C"))
    (for _array_element _outactors
      (Default|GameOver _array_element)
      (AddComponent|AddNiagaraComponent false))))

(event EventBeginPlay)

(event Collision|EventActorBeginOverlap
  (params (OtherActor :type Actor%20Object%20Reference)))

(event EventTick
  (params (DeltaSeconds :type Float%20%28single-precision%29)))

(event Input|ActionEvents|InputActionGrabEnemy
  (params (Key :type Key%20Structure :default "None"))
  (:Pressed
    (if (not (Variables|Default|GetbInAnimAttack))
      (if (Variables|Default|GetisGrabbingEnemy)
        (if (not (Variables|Default|GetbInAnimGrab))
          (Variables|Default|SetbInAnimGrab true)
          (bind _returnvalue (Animation|PlayAnimMontage "/Game/Characters/Ugly/MONTAGE_Ugly_Throw.MONTAGE_Ugly_Throw" 1.0 "None")) ; Throw
          (Utilities|FlowControl|Delay _returnvalue)
          (Variables|Default|SetbInAnimGrab false))
        (elif (not (Variables|Default|GetbInAnimThrow))
          (Variables|Default|SetbInAnimThrow true)
          (bind _returnvalue_2 (Animation|PlayAnimMontage "/Game/Characters/Ugly/MONTAGE_Ugly_Grab.MONTAGE_Ugly_Grab" 1.0 "None")) ; Grab
          (Utilities|FlowControl|Delay _returnvalue_2)
          (Variables|Default|SetbInAnimThrow false))))))

(event Input|ActionEvents|InputActionDash
  (params (Key :type Key%20Structure :default "None"))
  (:Pressed
    (Animation|Montage|PlayMontage 0 "/Game/Characters/Ugly/MONTAGE_Ugly_Dash.MONTAGE_Ugly_Dash" 0.0 0.48)))

(event Input|ActionEvents|InputActionThrowEnemy
  (params (Key :type Key%20Structure :default "None"))
  (:Pressed
    (if (not (Variables|Default|GetbInAnimAttack))
      (if (Variables|Default|GetisGrabbingEnemy)
        (if (not (Variables|Default|GetbInAnimGrab))
          (Variables|Default|SetbInAnimGrab true)
          (bind _returnvalue (Animation|PlayAnimMontage "/Game/Characters/Ugly/MONTAGE_Ugly_Throw.MONTAGE_Ugly_Throw" 1.0 "None")) ; Throw
          (Utilities|FlowControl|Delay _returnvalue)
          (Variables|Default|SetbInAnimGrab false))
        (elif (not (Variables|Default|GetbInAnimThrow))
          (Variables|Default|SetbInAnimThrow true)
          (bind _returnvalue_2 (Animation|PlayAnimMontage "/Game/Characters/Ugly/MONTAGE_Ugly_Grab.MONTAGE_Ugly_Grab" 1.0 "None")) ; Grab
          (Utilities|FlowControl|Delay _returnvalue_2)
          (Variables|Default|SetbInAnimThrow false))))))

(event Input|ActionEvents|InputActionMeleeAttack
  (params (Key :type Key%20Structure :default "None"))
  (bind _returnvalue (Transformation|GetActorLocation))
  (:Pressed
    (if (not (Variables|Default|GetbInAnimAttack))
      (Variables|Default|SetbInAnimAttack true)
      (bind _returnvalue_2 (Animation|PlayAnimMontage "/Game/Characters/Ugly/MONTAGE_Ugly_Punch.MONTAGE_Ugly_Punch" 1.0 "None"))
      (Utilities|FlowControl|Sequence
        (:then_0
          (Utilities|FlowControl|Delay 0.65)
          (bind (_outhit _returnvalue_3) (Collision|SphereTraceForObjects _returnvalue (+ _returnvalue (* (Math|Vector|GetForwardVector (Transformation|GetActorRotation)) 1.5e+02)) 1.2e+02 (Utilities|Array|MakeArray "ObjectTypeQuery3") false 0 "ForDuration"))
          (if _returnvalue_3
            (bind _asbp_canard_raciste (Utilities|Casting|CastToBP_CanardRaciste (.HitActor (Collision|BreakHitResult _outhit))))
            (Default|GetHit _asbp_canard_raciste)))
        (:then_1
          (Utilities|FlowControl|Delay _returnvalue_2)
          (Variables|Default|SetbInAnimAttack false))))))

(event Input|ActionEvents|InputActionJump
  (params (Key :type Key%20Structure :default "None"))
  (:Pressed
    (Animation|PlayAnimMontage 0 1.0 "None")))

(fn ConstructionScript)
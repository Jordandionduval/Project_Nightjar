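; BP_CanardLanceur is an AI duck enemy that picks up BP_CanardRaciste actors and throws them, and can also ram or attack.
; Pawn sensing and the DetectPlayer overlap write player flags to the Blackboard.
; Events handle carry and ram speeds, a sphere-trace attack that only swaps materials, and a montage-timed launch.
; FindClosest actually keeps the last duck found, as its distance comparison is unwired.
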(event OnSeePawn(PawnSensing)
  (params (Pawn :type Pawn%20Object%20Reference))
  (Utilities|Casting|CastToBP_FirstPersonCharacter Pawn)
  (AI|Components|Blackboard|SetValueasBool (AI|GetBlackboard (AI|GetAIController self)) (Utilities|Name|MakeLiteralName "hasSeenPlayer") true))

(event OnComponentBeginOverlap(DetectPlayer)
  (params (OverlappedComponent :type Primitive%20Component%20Object%20Reference) (OtherActor :type Actor%20Object%20Reference) (OtherComp :type Primitive%20Component%20Object%20Reference) (OtherBodyIndex :type Integer) (bFromSweep :type Boolean) (SweepResult :type Hit%20Result%20Structure%20%28by%20ref%29))
  (if (not (Variables|Default|GetIsinRange))
    (if (== (Utilities|GetClass OtherActor) "/Game/FPS_Template/FirstPerson/Blueprints/BP_FirstPersonCharacter.BP_FirstPersonCharacter_C")
      (Variables|Default|SetIsinRange true)
      (AI|Components|Blackboard|SetValueasBool (AI|GetBlackboard (AI|GetAIController self)) (Utilities|Name|MakeLiteralName "IsinRange") true))))

(event OnComponentEndOverlap(DetectPlayer)
  (params (OverlappedComponent :type Primitive%20Component%20Object%20Reference) (OtherActor :type Actor%20Object%20Reference) (OtherComp :type Primitive%20Component%20Object%20Reference) (OtherBodyIndex :type Integer))
  (if (Variables|Default|GetIsinRange)
    (if (== (Utilities|GetClass OtherActor) "/Game/FPS_Template/FirstPerson/Blueprints/BP_FirstPersonCharacter.BP_FirstPersonCharacter_C")
      (Variables|Default|SetIsinRange false)
      (AI|Components|Blackboard|SetValueasBool (AI|GetBlackboard (AI|GetAIController self)) (Utilities|Name|MakeLiteralName "IsinRange") false))))

(event Custom|Attack
  (bind _returnvalue (Transformation|GetActorLocation))
  (bind (_outhit _returnvalue_2) (Collision|SphereTraceForObjects _returnvalue (+ _returnvalue (* (Math|Vector|GetForwardVector (Transformation|GetActorRotation)) 2.5e+02)) 1.2e+02 (Utilities|Array|MakeArray "ObjectTypeQuery3") false 0 "ForDuration"))
  (if _returnvalue_2
    (Utilities|Casting|CastToBP_FirstPersonCharacter (.HitActor (Collision|BreakHitResult _outhit)))
    (Rendering|Material|SetMaterial (Variables|Character|GetMesh) 0 0)
    (Utilities|FlowControl|Delay 0.2)
    (Rendering|Material|SetMaterial (Variables|Character|GetMesh) 0 0)))

(event Custom|RamStop
  (Variables|/Script/Engine.CharacterMovementComponent|SetMaxWalkSpeed (Variables|Character|GetCharacterMovement) (Variables|Default|GetNormalSpeed))
  (Utilities|FlowControl|Delay 3.0)
  (AI|Components|Blackboard|SetValueasBool (AI|GetBlackboard (AI|GetAIController self)) (Utilities|Name|MakeLiteralName "hasSeenPlayer") false))

(event Custom|RamStart
  (Variables|/Script/Engine.CharacterMovementComponent|SetMaxWalkSpeed (Variables|Character|GetCharacterMovement) (Variables|Default|GetRamSpeed)))

(event Custom|FindClosest
  (bind _outactors (Actor|GetAllActorsOfClass "/Game/AI/BP_CanardRaciste.BP_CanardRaciste_C"))
  (for (_array_element _array_index) _outactors
    (if (== _array_index 0)
      (bind _output_get (Variables|Default|SetClosestCanard _array_element))
      (Collision|IgnoreActorwhenMoving (Variables|Collision|GetCapsuleComponent) _output_get true)
      (elif true
        (bind _output_get_2 (Variables|Default|SetClosestCanard _array_element))
        (Collision|IgnoreActorwhenMoving (Variables|Collision|GetCapsuleComponent) _output_get_2 true)))))

(event Custom|pickingUp
  (AI|Components|Blackboard|SetValueasBool (AI|GetBlackboard (AI|GetAIController self)) (Utilities|Name|MakeLiteralName "AsProjectile") true)
  (Variables|/Script/Engine.CharacterMovementComponent|SetMaxWalkSpeed (Variables|Character|GetCharacterMovement) (Variables|Default|GetCarrySpeed))
  (Variables|Default|Setcarry 1e+02))

(event Custom|YEET
  (Animation|PlayAnimMontage "/Game/Characters/Duck/AM_YEET.AM_YEET" 1.0 "None")
  (Utilities|FlowControl|Delay 1.0)
  (Default|GetThrown (Variables|Default|GetClosestCanard))
  (Character|LaunchCharacter (Variables|Default|GetClosestCanard) (* (Math|Vector|GetForwardVector (Transformation|GetActorRotation)) 1e+03) false false)
  (AI|Components|Blackboard|SetValueasBool (AI|GetBlackboard (AI|GetAIController self)) (Utilities|Name|MakeLiteralName "AsProjectile") false)
  (Variables|/Script/Engine.CharacterMovementComponent|SetMaxWalkSpeed (Variables|Character|GetCharacterMovement) (Variables|Default|GetNormalSpeed))
  (Variables|Default|Setcarry 0.0))

(event EventBeginPlay)

(event Collision|EventActorBeginOverlap
  (params (OtherActor :type Actor%20Object%20Reference)))

(event EventTick
  (params (DeltaSeconds :type Float%20%28single-precision%29)))

(fn ConstructionScript)
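; BP_spawner is an actor that repeatedly spawns BP_CanardRaciste actors at its SpawnPoint component's world transform.
; It spawns one on BeginPlay, then Tick drives a Delay with a random duration between MinCooldown and MaxCooldown before each further spawn.
; Spawns adjust for collisions but always happen, and the graph sets no limit on their count.
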(event EventBeginPlay
  (Game|SpawnActorfromClass "/Game/AI/BP_CanardRaciste.BP_CanardRaciste_C" (Transformation|GetWorldTransform (Variables|Default|GetSpawnPoint)) "AdjustIfPossibleButAlwaysSpawn" "MultiplyWithRoot" 0 0))

(event Collision|EventActorBeginOverlap
  (params (OtherActor :type Actor%20Object%20Reference)))

(event EventTick
  (params (DeltaSeconds :type Float%20%28single-precision%29))
  (Utilities|FlowControl|Delay (Math|Random|RandomFloatinRange (Variables|Default|GetMinCooldown) (Variables|Default|GetMaxCooldown)))
  (Game|SpawnActorfromClass "/Game/AI/BP_CanardRaciste.BP_CanardRaciste_C" (Transformation|GetWorldTransform (Variables|Default|GetSpawnPoint)) "AdjustIfPossibleButAlwaysSpawn" "MultiplyWithRoot" 0 0))

(fn ConstructionScript)
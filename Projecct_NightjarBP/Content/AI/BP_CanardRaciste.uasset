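; BP_CanardRaciste is an AI duck enemy that rams, punches, and can be carried and thrown by a CanardLanceur.
; Pawn sensing, a range overlap and pickup events set blackboard flags; ramming changes walk speed, then sets Dizzy.
; Attacks alternate two punch montages with delayed sphere traces, though hits apply no damage and zero HitCount triggers nothing.
; While caught, it switches to flying and follows the carrier's PositionCaught every tick.
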(event OnSeePawn(PawnSensing)
  (params (Pawn :type Pawn%20Object%20Reference))
  ;[1 1 1] Sense player
  (Utilities|Casting|CastToBP_FirstPersonCharacter Pawn)
  (AI|Components|Blackboard|SetValueasBool (AI|GetBlackboard (AI|GetAIController self)) (Utilities|Name|MakeLiteralName "hasSeenPlayer") true))

(event OnComponentBeginOverlap(DetectPlayer)
  (params (OverlappedComponent :type Primitive%20Component%20Object%20Reference) (OtherActor :type Actor%20Object%20Reference) (OtherComp :type Primitive%20Component%20Object%20Reference) (OtherBodyIndex :type Integer) (bFromSweep :type Boolean) (SweepResult :type Hit%20Result%20Structure%20%28by%20ref%29))
  ;[1 1 1] Check si le joueur est dans son range d'attaque
  (if (not (Variables|Default|GetIsinRange))
    (if (== (Utilities|GetClass OtherActor) "/Game/FPS_Template/FirstPerson/Blueprints/BP_FirstPersonCharacter.BP_FirstPersonCharacter_C")
      (Variables|Default|SetIsinRange true)
      (AI|Components|Blackboard|SetValueasBool (AI|GetBlackboard (AI|GetAIController self)) (Utilities|Name|MakeLiteralName "IsinRange") true))))

(event OnComponentEndOverlap(DetectPlayer)
  (params (OverlappedComponent :type Primitive%20Component%20Object%20Reference) (OtherActor :type Actor%20Object%20Reference) (OtherComp :type Primitive%20Component%20Object%20Reference) (OtherBodyIndex :type Integer))
  ;[1 1 1] Check si le joueur est dans son range d'attaque
  (if (Variables|Default|GetIsinRange)
    (if (== (Utilities|GetClass OtherActor) "/Game/FPS_Template/FirstPerson/Blueprints/BP_FirstPersonCharacter.BP_FirstPersonCharacter_C")
      (Variables|Default|SetIsinRange false)
      (AI|Components|Blackboard|SetValueasBool (AI|GetBlackboard (AI|GetAIController self)) (Utilities|Name|MakeLiteralName "IsinRange") false))))

(event Custom|Attack
  (bind _returnvalue (Transformation|GetActorLocation))
  (bind _returnvalue_2 (Transformation|GetActorLocation))
  ;[1 1 1] attack
  (Utilities|FlowControl|Delay 1.0)
  (if (Variables|Default|GetIsinRange)
    (Utilities|FlowControl|FlipFlop
      (:A
        (Animation|PlayAnimMontage "/Game/Characters/Duck/AM_DuckPunch.AM_DuckPunch" 1.0 "None")
        (Utilities|FlowControl|Delay 0.65)
        (bind (_outhit _returnvalue_3) (Collision|SphereTraceForObjects _returnvalue_2 (+ _returnvalue_2 (* (Math|Vector|GetForwardVector (Transformation|GetActorRotation)) 1.5e+02)) 1.2e+02 (Utilities|Array|MakeArray "ObjectTypeQuery3") false 0 "ForDuration"))
        (if _returnvalue_3
          (Utilities|Casting|CastToBP_FirstPersonCharacter (.HitActor (Collision|BreakHitResult _outhit)))))
      (:B
        (Animation|PlayAnimMontage "/Game/Characters/Duck/AM_DuckPunch2.AM_DuckPunch2" 1.0 "None")
        (Utilities|FlowControl|Delay 0.6)
        (bind (_outhit_2 _returnvalue_4) (Collision|SphereTraceForObjects _returnvalue (+ _returnvalue (* (Math|Vector|GetForwardVector (Transformation|GetActorRotation)) 1.5e+02)) 1.2e+02 (Utilities|Array|MakeArray "ObjectTypeQuery3") false 0 "ForDuration"))
        (if _returnvalue_4
          (Utilities|Casting|CastToBP_FirstPersonCharacter (.HitActor (Collision|BreakHitResult _outhit_2))))))))

(event Custom|RamStop
  ;[1 1 1] Foncer sur player
  (Variables|/Script/Engine.CharacterMovementComponent|SetMaxWalkSpeed (Variables|Character|GetCharacterMovement) (Variables|Default|GetNormalSpeed))
  (Variables|Default|Setdizzy 1e+02)
  (Utilities|FlowControl|Delay 3.0)
  (AI|Components|Blackboard|SetValueasBool (AI|GetBlackboard (AI|GetAIController self)) (Utilities|Name|MakeLiteralName "hasSeenPlayer") false))

(event Custom|RamStart
  ;[1 1 1] Foncer sur player
  (Variables|/Script/Engine.CharacterMovementComponent|SetMaxWalkSpeed (Variables|Character|GetCharacterMovement) (Variables|Default|GetRamSpeed)))

(event Custom|StopDizzy
  ;[1 1 1] Foncer sur player
  (Variables|Default|Setdizzy 0.0))

(event Custom|getPickedUp
  (params (CanardLanceur :type BP%20Canard%20Lanceur%20Object%20Reference))
  ;[1 1 1] go on head of canard lanceur
  (AI|Components|Blackboard|SetValueasBool (AI|GetBlackboard (AI|GetAIController self)) (Utilities|Name|MakeLiteralName "IsCaught") true)
  (Variables|Default|SetCanard%20Lanceur CanardLanceur)
  (Pawn|Components|CharacterMovement|SetMovementMode (Variables|Character|GetCharacterMovement) "MOVE_Flying" 0)
  (Transformation|SetActorLocation (Transformation|GetWorldLocation (Variables|/Game/AI/BP_CanardLanceur.BP_CanardLanceur_C|GetpositionCaught CanardLanceur)) false true)
  (Variables|Default|SetIsStuck true))

(event Custom|GetHit
  ;[1 1 1] attack
  (Variables|Default|SethitCount (- (Variables|Default|GethitCount) 1))
  (bind _returnvalue (Animation|PlayAnimMontage "/Game/Characters/Duck/AM_Hit.AM_Hit" 1.0 "None"))
  (Utilities|FlowControl|Delay _returnvalue)
  (if (== (Variables|Default|GethitCount) 0)
    _))

(event Custom|GetThrown
  ;[1 1 1] Getting thrown
  (AI|Components|Blackboard|SetValueasBool (AI|GetBlackboard (AI|GetAIController self)) (Utilities|Name|MakeLiteralName "IsCaught") false)
  (Variables|Default|SetIsStuck false)
  (AI|Components|Blackboard|SetValueasBool (AI|GetBlackboard (AI|GetAIController self)) (Utilities|Name|MakeLiteralName "hasSeenPlayer") false))

(event EventBeginPlay)

(event Collision|EventActorBeginOverlap
  (params (OtherActor :type Actor%20Object%20Reference)))

(event EventTick
  (params (DeltaSeconds :type Float%20%28single-precision%29))
  (if (Variables|Default|GetIsStuck)
    (Transformation|SetActorLocation (Transformation|GetWorldLocation (Variables|/Game/AI/BP_CanardLanceur.BP_CanardLanceur_C|GetpositionCaught (Variables|Default|GetCanard%20Lanceur))) true false)))

(fn ConstructionScript)
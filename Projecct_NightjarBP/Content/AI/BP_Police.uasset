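; BP_Police is an animated spawner that periodically releases BP_CanardRaciste actors while CanSpawn is true.
; Tick drives the cycle through a Delay of random length between MinCooldown and MaxCooldown.
; It then plays the open montage, waits for that montage's returned duration, spawns the actor at SpawnPoint and plays the closed montage.
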(event EventBeginPlay)

(event Collision|EventActorBeginOverlap
  (params (OtherActor :type Actor%20Object%20Reference)))

(event EventTick
  (params (DeltaSeconds :type Float%20%28single-precision%29))
  (if (Variables|Default|GetbCanSpawn)
    (Utilities|FlowControl|Delay (Math|Random|RandomFloatinRange (Variables|Default|GetMinCooldown) (Variables|Default|GetMaxCooldown)))
    (bind _returnvalue (Animation|PlayAnimMontage "/Game/Characters/Pollice/AM_PoliceOpen.AM_PoliceOpen" 1.0 "None"))
    (Utilities|FlowControl|Delay _returnvalue)
    (Game|SpawnActorfromClass "/Game/AI/BP_CanardRaciste.BP_CanardRaciste_C" (Transformation|GetWorldTransform (Variables|Default|GetSpawnPoint)) "AdjustIfPossibleButAlwaysSpawn" "MultiplyWithRoot" 0 0)
    (Animation|PlayAnimMontage "/Game/Characters/Pollice/AM_PoliceClosed.AM_PoliceClosed" 1.0 "None")))

(fn ConstructionScript)